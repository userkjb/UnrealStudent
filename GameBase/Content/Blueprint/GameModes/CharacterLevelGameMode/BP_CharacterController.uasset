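; Player controller for the character level game mode, routing Enhanced Input for movement, mouse look, dash and shooting.
; Move, pitch/yaw rotation and dash start/end are delegated to functions defined outside these graphs.
; Left-click firing only prints debug text, using ShotMode and an IsEnd held flag to gate a delayed repeat.
; An unconnected spring-arm rotation experiment, noted as not working, remains in the graph.
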(event Input|EnhancedActionEvents|EnhancedInputActionIA_MouseLeftButton
  (params (ActionValue :type Boolean) (ElapsedSeconds :type Float%20%28double-precision%29) (TriggeredSeconds :type Float%20%28double-precision%29) (InputAction :type Input%20Action%20Object%20Reference :default "/Game/Blueprint/Input/IA_MouseLeftButton.IA_MouseLeftButton"))
  ;[1 1 1] 총알
  (:Triggered
    ;;[1 1 1] 연발
    ;;;[1 1 1] 연발 / 단발
    (if (not (Variables|Default|GetShotMode))
      (Utilities|FlowControl|Delay 0.5)
      ;;;[1 1 1] End 후 또 들어 오는 현상 방지.
      (if (Variables|Default|GetIsEnd)
        (Development|PrintString "Tick"))))
  (:Started
    ;;[1 1 1] 시작
    (Development|PrintString "Start")
    (Variables|Default|SetIsEnd true) ; True
  )
  (:Completed
    ;;[1 1 1] 코멘트
    (Development|PrintString "End")
    (Variables|Default|SetIsEnd false) ; False
  ))

(event Input|EnhancedActionEvents|EnhancedInputActionIA_Run
  (params (ActionValue :type Boolean) (ElapsedSeconds :type Float%20%28double-precision%29) (TriggeredSeconds :type Float%20%28double-precision%29) (InputAction :type Input%20Action%20Object%20Reference :default "/Game/Blueprint/Input/IA_Run.IA_Run"))
  ;[1 1 1] 대쉬
  (:Started
    (Class|CharacterPlayerController|PlayerDashStart))
  (:Completed
    (Class|CharacterPlayerController|PlayerDashEnd)))

(event Input|EnhancedActionEvents|EnhancedInputActionIA_Mouse
  (params (ActionValue :type Vector%202D%20Structure) (ElapsedSeconds :type Float%20%28double-precision%29) (TriggeredSeconds :type Float%20%28double-precision%29) (InputAction :type Input%20Action%20Object%20Reference :default "/Game/Blueprint/Input/IA_Mouse.IA_Mouse"))
  ;[1 1 1] 마우스 회전
  (Class|CharacterPlayerController|PlayerPitchRotation ActionValue)
  (Class|CharacterPlayerController|PlayerYawRotation ActionValue))

(event Input|EnhancedActionEvents|EnhancedInputActionIA_Move
  (params (ActionValue :type Vector :default "0, 0, 0") (ElapsedSeconds :type Float%20%28double-precision%29) (TriggeredSeconds :type Float%20%28double-precision%29) (InputAction :type Input%20Action%20Object%20Reference :default "/Game/Blueprint/Input/IA_Move.IA_Move"))
  (Class|CharacterPlayerController|PlayerMoving ActionValue))

(event EventBeginPlay)

(event EventTick
  (params (DeltaSeconds :type Float%20%28single-precision%29)))

(fn ConstructionScript)