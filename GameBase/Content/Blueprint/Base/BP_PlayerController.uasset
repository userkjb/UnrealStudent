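; Base player controller that turns Enhanced Input actions into camera look and player movement commands.
; Mouse input is normalized, scaled by frame delta time and RotSpeed, then applied as yaw and pitch, so only its direction affects turn rate.
; Move input calls PlayerMove with MoveSpeed, while run press and release call PlayerRunIn and PlayerRunOut, none of which are defined in this graph.
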(event Input|EnhancedActionEvents|EnhancedInputActionIA_Mouse
  (params (ActionValue :type Vector%202D%20Structure) (ElapsedSeconds :type Float%20%28double-precision%29) (TriggeredSeconds :type Float%20%28double-precision%29) (InputAction :type Input%20Action%20Object%20Reference :default "/Game/Blueprint/Input/IA_Mouse.IA_Mouse"))
  (bind _returnvalue (Utilities|Time|GetWorldDeltaSeconds))
  (bind _returnvalue_2 (Math|Vector2D|Normalize2D ActionValue))
  (bind _self self)
  (bind _rotspeed (Variables|Default|GetRotSpeed))
  (bind (_x _y) (Math|Vector2D|BreakVector2D _returnvalue_2))
  (Utilities|FlowControl|Sequence
    (:then_1
      (Class|PlayerController|AddYawInput _self (* _x _returnvalue _rotspeed))
      (Class|PlayerController|AddPitchInput _self (* _y _returnvalue _rotspeed)))))

(event Input|EnhancedActionEvents|EnhancedInputActionIA_Run
  (params (ActionValue :type Boolean) (ElapsedSeconds :type Float%20%28double-precision%29) (TriggeredSeconds :type Float%20%28double-precision%29) (InputAction :type Input%20Action%20Object%20Reference :default "/Game/Blueprint/Input/IA_Run.IA_Run"))
  (:Started
    (Class|BasePlayerController|PlayerRunin))
  (:Completed
    (Class|BasePlayerController|PlayerRunOut)))

(event Input|EnhancedActionEvents|EnhancedInputActionIA_Move
  (params (ActionValue :type Vector :default "0, 0, 0") (ElapsedSeconds :type Float%20%28double-precision%29) (TriggeredSeconds :type Float%20%28double-precision%29) (InputAction :type Input%20Action%20Object%20Reference :default "/Game/Blueprint/Input/IA_Move.IA_Move"))
  (Class|BasePlayerController|PlayerMove ActionValue (Variables|Default|GetMoveSpeed)))

(event EventBeginPlay)

(event EventTick
  (params (DeltaSeconds :type Float%20%28single-precision%29)))

(fn ConstructionScript)